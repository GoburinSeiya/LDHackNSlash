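; BP_MovingPlat is a platform that moves while the player overlaps its Button and returns when they leave.
; BeginPlay applies an override material to both Platform and Button and stores the platform's starting relative location.
; Button overlaps, filtered by a player-check message on the other actor, play or reverse the MovePlatform timeline, which lerps the platform between start and target positions without sweeping.
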(event OnComponentBeginOverlap(Button)
  (params (OverlappedComponent :type Primitive%20Component%20Object%20Reference) (OtherActor :type Actor%20Object%20Reference) (OtherComp :type Primitive%20Component%20Object%20Reference) (OtherBodyIndex :type Integer) (bFromSweep :type Boolean) (SweepResult :type Hit%20Result%20Structure%20%28by%20ref%29))
  (bind _isplayer (Class|BPIPlayer|CheckIsPlayer(Message) OtherActor))
  (if _isplayer
    (bind _progress (Timeline|MovePlatform Play)
      (:Update
        (Transformation|SetRelativeLocation (Variables|Default|GetPlatform) (Math|Vector|Lerp(Vector) (Variables|Default|GetstartPos) (Variables|Default|GettargetPos) _progress) false false)))))

(event OnComponentEndOverlap(Button)
  (params (OverlappedComponent :type Primitive%20Component%20Object%20Reference) (OtherActor :type Actor%20Object%20Reference) (OtherComp :type Primitive%20Component%20Object%20Reference) (OtherBodyIndex :type Integer))
  (bind _isplayer (Class|BPIPlayer|CheckIsPlayer(Message) OtherActor))
  (if _isplayer
    (bind _progress (Timeline|MovePlatform Reverse)
      (:Update
        (Transformation|SetRelativeLocation (Variables|Default|GetPlatform) (Math|Vector|Lerp(Vector) (Variables|Default|GetstartPos) (Variables|Default|GettargetPos) _progress) false false)))))

(event EventBeginPlay
  (bind _materialoverwrite (Variables|Default|GetmaterialOverwrite))
  (Rendering|Material|SetMaterial (Variables|Default|GetPlatform) 0 _materialoverwrite)
  (Rendering|Material|SetMaterial (Variables|Default|GetButton) 0 _materialoverwrite)
  (Variables|Default|SetstartPos (Variables|/Script/Engine.SceneComponent|GetRelativeLocation (Variables|Default|GetPlatform))))

(fn ConstructionScript)
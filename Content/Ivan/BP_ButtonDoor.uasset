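; Button-operated door that sinks the Wall while a player overlaps the Cube and raises it again when the player leaves.
; BeginPlay applies an override material to one slot on each mesh and caches the Wall's starting relative location.
; Overlap events confirm the player through a CheckIsPlayer message, then play or reverse the MoveDoor timeline, which lerps the Wall's height down by a fixed distance.
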(event OnComponentBeginOverlap(Cube)
  (params (OverlappedComponent :type Primitive%20Component%20Object%20Reference) (OtherActor :type Actor%20Object%20Reference) (OtherComp :type Primitive%20Component%20Object%20Reference) (OtherBodyIndex :type Integer) (bFromSweep :type Boolean) (SweepResult :type Hit%20Result%20Structure%20%28by%20ref%29))
  (bind _startposition (Variables|Default|GetstartPosition))
  (bind _isplayer (Class|BPIPlayer|CheckIsPlayer(Message) OtherActor))
  (if _isplayer
    (bind _progress (Timeline|MoveDoor Play)
      (:Update
        (Transformation|SetRelativeLocation (Variables|Default|GetWall) (Math|Vector|MakeVector (.x _startposition) (.y _startposition) (Math|Float|Lerp (.z _startposition) (- (.z _startposition) 9e+02) _progress)) false false)))))

(event OnComponentEndOverlap(Cube)
  (params (OverlappedComponent :type Primitive%20Component%20Object%20Reference) (OtherActor :type Actor%20Object%20Reference) (OtherComp :type Primitive%20Component%20Object%20Reference) (OtherBodyIndex :type Integer))
  (bind _startposition (Variables|Default|GetstartPosition))
  (bind _isplayer (Class|BPIPlayer|CheckIsPlayer(Message) OtherActor))
  (if _isplayer
    (bind _progress (Timeline|MoveDoor Reverse)
      (:Update
        (Transformation|SetRelativeLocation (Variables|Default|GetWall) (Math|Vector|MakeVector (.x _startposition) (.y _startposition) (Math|Float|Lerp (.z _startposition) (- (.z _startposition) 9e+02) _progress)) false false)))))

(event EventBeginPlay
  (bind _materialoverwrite (Variables|Default|GetmaterialOverwrite))
  (Rendering|Material|SetMaterial (Variables|Default|GetCube) 0 _materialoverwrite)
  (Rendering|Material|SetMaterial (Variables|Default|GetWall) 1 _materialoverwrite)
  (Variables|Default|SetstartPosition (Variables|/Script/Engine.SceneComponent|GetRelativeLocation (Variables|Default|GetWall))))

(fn ConstructionScript)